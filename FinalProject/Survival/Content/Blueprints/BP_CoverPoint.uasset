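; Cover point actor that tracks whether an AI enemy tank is occupying it.
; When an actor tagged AI begins overlapping, it marks itself taken, stores that EnemyTank and sets itself as the tank's current cover point.
; When the overlap ends, it marks itself free and resets both references to null placeholder variables.
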(event EventBeginPlay)

(event Collision|EventActorBeginOverlap
  (params (OtherActor :type Actor%20Object%20Reference))
  (if (Actor|ActorHasTag OtherActor "AI")
    (Variables|Default|SetCoverPointFree false)
    (bind _asenemy_tank (Utilities|Casting|CastToEnemyTank OtherActor))
    (Variables|Default|SetColliding%20Tank _asenemy_tank)
    (bind _asenemy_tank_2 (Utilities|Casting|CastToEnemyTank OtherActor))
    (Variables|/Script/Survival.EnemyTank|SetCurrentCoverPoint _asenemy_tank_2 self)))

(event Collision|EventActorEndOverlap
  (params (OtherActor :type Actor%20Object%20Reference))
  (if (Actor|ActorHasTag OtherActor "AI")
    (Variables|Default|SetCoverPointFree true)
    (Variables|Default|SetColliding%20Tank (Variables|Default|GetNull%20Tank))
    (bind _asenemy_tank (Utilities|Casting|CastToEnemyTank OtherActor))
    (Variables|/Script/Survival.EnemyTank|SetCurrentCoverPoint _asenemy_tank (Variables|Default|GetNull%20Actor))))

(fn ConstructionScript)