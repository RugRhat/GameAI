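; BP_SurvivalGM is a game mode Blueprint, apparently for a tank survival mode, that handles game over and cover point availability.
; Its GameOver event creates the WBP_GameEnd widget, adds it to the viewport and calls GameEndReady on it.
; IsCoverPointFree reports a BP_CoverPoint as free if it is flagged free or if the querying enemy tank is the one colliding with it.
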(event EventBeginPlay)

(event EventGameOver
  (bind _returnvalue (UserInterface|CreateWidget "/Game/Widgets/WBP_GameEnd.WBP_GameEnd_C"))
  (UserInterface|Viewport|AddtoViewport _returnvalue 0)
  (Default|GameEndReady _returnvalue))

(fn ConstructionScript)

(fn IsCoverPointFree
  (params (CoverPoint :type Actor%20Object%20Reference) (EnemyTank :type Enemy%20Tank%20Object%20Reference))
  (bind _asbp_cover_point (Utilities|Casting|CastToBP_CoverPoint CoverPoint))
  (if (Variables|/Game/Blueprints/BP_CoverPoint.BP_CoverPoint_C|GetCoverPointFree _asbp_cover_point)
    (Variables|Default|SetPoint%20Free true)
    (elif (== EnemyTank (Variables|/Game/Blueprints/BP_CoverPoint.BP_CoverPoint_C|GetColliding%20Tank _asbp_cover_point))
      (Variables|Default|SetPoint%20Free true)
      (else
        (Variables|Default|SetPoint%20Free false))))
  (return (Variables|Default|GetPoint%20Free)))